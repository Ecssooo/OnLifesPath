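; BP_PlaySoundMenu plays the menu music and provides a fade-out for it.
; On BeginPlay it passes its sound list and audio component to the SoundManager as a playlist, then binds to the MenuManager's Play dispatcher.
; A custom fade-out event runs a timeline that drives the audio component's volume level on each update.
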(event `self.ReceiveBeginPlay`
  (`SoundManager.SoundPlaylist` (subsystem `SoundManager`) (`self.SoundList`) (`self.Audio`))
  (add `/Game/UI/Menu/BP_MenuManager.ED_Play` (`self.MenuManager`) (`|CreateDelegate` :!event `CE_FadeMusicOut`)))

(event `CE_FadeMusicOut`
  (bind (_direction _fadeout) (`Timeline|FadeMusicOut` :!via `PlayFromStart`)
    (:`Update`
      (`AudioComponent.AdjustVolume` (`self.Audio`) 0.0 _fadeout "Linear"))))

(fn `UserConstructionScript`)