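; BP_Spectator provides free-fly spectator controls by driving a BP_CameraActor found in the level rather than moving itself.
; On BeginPlay it caches that camera and turns off its CanFollow flag, which fly input also clears.
; Enhanced Input look adds to the camera's pitch and yaw, while fly offsets it along its local axes at a fixed step per event, without sweep or delta-time scaling.
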(event `self.ReceiveBeginPlay`
  (bind _returnvalue (`GameplayStatics.GetActorOfClass` "/Game/BP/Camera/BP_CameraActor.BP_CameraActor_C"))
  (bind _output_get (set `self.Camera` _returnvalue))
  (set `/Game/BP/Camera/BP_CameraActor.CanFollow` false _output_get))

(event `EnhancedInput|/Game/Input/IA/Spectator/IA_Look`
  (params (ActionValue :type "Vector2D Structure") (ElapsedSeconds :type "Float (double-precision)") (TriggeredSeconds :type "Float (double-precision)") (InputAction :type "InputAction Object Reference" :default "/Game/Input/IA/Spectator/IA_Look.IA_Look"))
  (bind (_returnvalue_roll _returnvalue_pitch _returnvalue_yaw) (`KismetMathLibrary.BreakRotator` (`self.K2_GetActorRotation` (`self.Camera`))))
  (:`Triggered`
    (`self.K2_SetActorRotation` (`self.Camera`) (`KismetMathLibrary.MakeRotator` 0.0 (+ ActionValue_Y _returnvalue_pitch) (+ ActionValue_X _returnvalue_yaw)) false)))

(event `EnhancedInput|/Game/Input/IA/Spectator/IA_Fly`
  (params (ActionValue :type "Vector Structure") (ElapsedSeconds :type "Float (double-precision)") (TriggeredSeconds :type "Float (double-precision)") (InputAction :type "InputAction Object Reference" :default "/Game/Input/IA/Spectator/IA_Fly.IA_Fly"))
  (bind _camera (`self.Camera`))
  (:`Triggered`
    (set `/Game/BP/Camera/BP_CameraActor.CanFollow` false (`self.Camera`))
    (`self.K2_SetActorLocation` (`self.Camera`) (+ (* (+ (* ActionValue_X (`self.GetActorForwardVector` (`self.Camera`))) (* ActionValue_Y (`self.GetActorRightVector` _camera)) (* ActionValue_Z (`self.GetActorUpVector` _camera))) 5.0) (`self.K2_GetActorLocation` (`self.Camera`))) false false)))

(fn `UserConstructionScript`)