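; BP_IntroCinematic is a step that plays the intro cinematic as a slideshow of textures with matching text.
; On start it creates a WBP_Cinematic widget, then a self-calling event steps through the image array using timed delays.
; Fade timelines drive the widget's fade opacity, swapping image and text while the screen is black.
; After the last image it fades, advances the StepManager, and removes the widget when the step ends.
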(event `CE_DoCinematic`
  ; DoCinematic
  (if (< (`self.TextureCinematicIndex`) (`KismetArrayLibrary.Array_Length` (`self.CinematicTexture`)))
    (`self.CE_FadeIn` (`|GetArrayItem` (`self.CinematicTexture`) (`self.TextureCinematicIndex`)) true)
    (`KismetSystemLibrary.Delay` (`self.ImageCinematicDuration`))
    (`/Engine/EditorBlueprintResources/StandardMacros.IncrementInt` (`self.TextureCinematicIndex`)
      (:`  `
        (`self.CE_DoCinematic`)))
    (else
      (`self.CE_FadeIn` null)
      (`KismetSystemLibrary.Delay` (`self.FadeInEnd`))
      (`StepManager.NextStep` (`self.StepManager`)))))

(event `self.OnStartStep`
  ; StartSetp
  (bind _returnvalue (`|CreateWidget` "/Game/BP/Steps/Cinematics/WBP_Cinematic.WBP_Cinematic_C"))
  (bind _output_get (set `self.CinematicWidget` _returnvalue))
  (`UserWidget.AddToViewport` _output_get 0)
  (`self.CE_SetupWidget`)
  (`KismetSystemLibrary.Delay` (`self.FadeInStart`))
  (`self.CE_DoCinematic`))

(event `self.OnEndStep`
  ; EndStep
  (`Widget.RemoveFromParent` (`self.CinematicWidget`)))

(event `CE_SetupWidget`
  (bind _cinematicwidget (`self.CinematicWidget`))
  (`/Game/BP/Steps/Cinematics/WBP_Cinematic.CE_SetNextTexture` _cinematicwidget (`|GetArrayItem` (`self.CinematicTexture`)))
  (`/Game/BP/Steps/Cinematics/WBP_Cinematic.CE_SetText` _cinematicwidget (`|GetArrayItem` (`self.CinematicText`))))

(event `CE_FadeIn`
  (params (Texture :type "Texture2D Object Reference") (DoTransition :type Boolean))
  ; FadeIn
  (bind (_direction _opac) (`Timeline|FadeIn` :!via `PlayFromStart`)
    (:`Update`
      (`/Game/BP/Steps/Cinematics/WBP_Cinematic.CE_SetFadeOpacity` (`self.CinematicWidget`) _opac))
    (:`Finished`
      (if DoTransition
        (`/Game/BP/Steps/Cinematics/WBP_Cinematic.CE_SetNextTexture` (`self.CinematicWidget`) Texture)
        (`/Game/BP/Steps/Cinematics/WBP_Cinematic.CE_SetText` (`self.CinematicWidget`) (`|GetArrayItem` (`self.CinematicText`) (`self.TextureCinematicIndex`)))
        (`KismetSystemLibrary.Delay` (`self.BlackScreenDuration`))
        (`self.CE_FadeOut`)))))

(event `CE_FadeOut`
  ; FadeOut
  (bind (_direction _opac) (`Timeline|FadeOut` :!via `PlayFromStart`)
    (:`Update`
      (`/Game/BP/Steps/Cinematics/WBP_Cinematic.CE_SetFadeOpacity` (`self.CinematicWidget`) _opac))))

(fn `GetNextTexture`
  (returns (Texture :type "Texture2D Object Reference"))
  (return (`|GetArrayItem` (`self.CinematicTexture`) (`self.TextureCinematicIndex`))))

(fn `UserConstructionScript`)